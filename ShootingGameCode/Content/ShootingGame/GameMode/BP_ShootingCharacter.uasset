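; BP_ShootingCharacter is the shooting game's character Blueprint, connecting the character to its NameTagWidget.
; An update event passes the mesh's "nametag" socket location to the widget to update the tag's position.
; HP and name update events call their parent implementations, then forward the values to the widget, casting NameTagWidget before each call.
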(event `self.EventUpdateNameTag`
  (bind _asname_tag_widget (cast `/Game/ShootingGame/Widget/NameTagWidget` (`self.NameTagWidget`)))
  (`/Game/ShootingGame/Widget/NameTagWidget.UpdateNameTagPosition` _asname_tag_widget (`SceneComponent.GetSocketLocation` (`self.Mesh`) "nametag")))

(event `self.OnUpdateHp`
  (params (CurHp :type "Float (single-precision)") (MaxHp :type "Float (single-precision)"))
  (`parent.OnUpdateHp` CurHp MaxHp)
  (bind _asname_tag_widget (cast `/Game/ShootingGame/Widget/NameTagWidget` (`self.NameTagWidget`)))
  (`/Game/ShootingGame/Widget/NameTagWidget.SetHp` _asname_tag_widget CurHp MaxHp))

(event `self.OnUpdateUserNametag`
  (params (name :type String))
  (`parent.OnUpdateUserNametag` name)
  (bind _asname_tag_widget (cast `/Game/ShootingGame/Widget/NameTagWidget` (`self.NameTagWidget`)))
  (`/Game/ShootingGame/Widget/NameTagWidget.SetPlayerName` _asname_tag_widget name))

(fn `UserConstructionScript`)