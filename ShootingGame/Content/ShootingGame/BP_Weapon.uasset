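; Networked, data-driven gun for the shooting game that characters can pick up, drop, fire and reload.
; WeaponData supplies mesh, montages, effects, damage and starting ammo.
; EventShoot plays muzzle effects, and the local player passes camera aim to server-side ReqShoot, which spends ammo, line-traces from past the spring arm and damages hit Characters.
; OnRep Ammo, pickup and drop update the owning local player's BP_ShootingHUD.
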(event `ReqShoot`
  (params (StartLocation :type "Vector Structure") (ForwardLocation :type "Vector Structure"))
  (bind (_weapondata_staticmesh _weapondata_shootmontage _weapondata_reloadmontage _weapondata_soundbase _weapondata_fireeffet _weapondata_maxammo _weapondata_damage) (break `/Game/ShootingGame/ST_Weapon` (`self.WeaponData`)))
  ;[1 1 1 1 16] 서버에서 전달받는 Location
  (bind _isused (`self.UseAmmo`))
  (if _isused
    (bind (_outhit _returnvalue) (`KismetSystemLibrary.LineTraceSingleForObjects` :`Start` (+ StartLocation (* ForwardLocation (`self.GetFireStartLength`))) :`End` (+ StartLocation (* ForwardLocation 5000.0)) :`ObjectTypes` (`|MakeArray` "ObjectTypeQuery1" "ObjectTypeQuery2" "ObjectTypeQuery3" "ObjectTypeQuery4" "ObjectTypeQuery5" "ObjectTypeQuery6" :!type "EObjectTypeQuery Enum") :`DrawDebugType` "Persistent"))
    (if _returnvalue
      (bind `_as캐릭터` (cast `Character` (`.HitActor` (`GameplayStatics.BreakHitResult` _outhit))))
      (`GameplayStatics.ApplyDamage` `_as캐릭터` _weapondata_damage (`Pawn.GetController` (`self.OwnChar`)) self))))

(event `self.ReceiveBeginPlay`
  (bind (_weapondata_staticmesh _weapondata_shootmontage _weapondata_reloadmontage _weapondata_soundbase _weapondata_fireeffet _weapondata_maxammo) (break `/Game/ShootingGame/ST_Weapon` (`self.WeaponData`)))
  (`StaticMeshComponent.SetStaticMesh` (`self.StaticMesh`) _weapondata_staticmesh)
  (set `self.Ammo` (`KismetMathLibrary.Conv_IntToByte` _weapondata_maxammo)))

(fn `EventDrop`
  (params (Char :type "Character Object Reference"))
  (returns (bResult :type Boolean))
  (bind _staticmesh (`self.StaticMesh`))
  ;[1 1 1 1 16] OwnChar가 비어지기 전에 처리해야함
  (`self.UpdateMyAmmo` 0)
  (set `self.OwnChar` null)
  (`PrimitiveComponent.SetSimulatePhysics` _staticmesh true)
  (`SceneComponent.K2_DetachFromComponent` _staticmesh "KeepWorld" "KeepWorld" "KeepWorld" true)
  (return false))

(fn `EventPickUp`
  (params (Character :type "Character Object Reference"))
  (returns (bResult :type Boolean))
  (bind _output_get (set `self.OwnChar` Character))
  (`PrimitiveComponent.SetSimulatePhysics` (`self.StaticMesh`) false)
  (`self.K2_AttachToComponent` self (`Character.Mesh` _output_get) "weapon" "SnapToTarget" "SnapToTarget" "KeepWorld" true)
  (`self.UpdateMyAmmo` (`self.Ammo`))
  (return false))

(fn `EventReload`
  (returns (bResult :type Boolean))
  (bind (_weapondata_staticmesh _weapondata_shootmontage _weapondata_reloadmontage) (break `/Game/ShootingGame/ST_Weapon` (`self.WeaponData`)))
  (`Character.PlayAnimMontage` (`self.OwnChar`) _weapondata_reloadmontage 1.0 "None")
  (return true))

(fn `EventResetAmmo`
  (returns (bResult :type Boolean))
  (`self.SetAmmo` 30)
  (return true))

(fn `EventShoot`
  (returns (bResult :type Boolean))
  (bind _returnvalue (`GameplayStatics.GetPlayerCameraManager` 0))
  (bind _staticmesh (`self.StaticMesh`))
  (bind (_weapondata_staticmesh _weapondata_shootmontage _weapondata_reloadmontage _weapondata_soundbase _weapondata_fireeffet) (break `/Game/ShootingGame/ST_Weapon` (`self.WeaponData`)))
  (bind _returnvalue_2 (`SceneComponent.GetSocketLocation` _staticmesh "Muzzle"))
  (if (`self.IsCanShoot`)
    (`GameplayStatics.SpawnEmitterAtLocation` _weapondata_fireeffet _returnvalue_2 (`SceneComponent.GetSocketRotation` _staticmesh "Muzzle") (0.1 0.1 0.1))
    (`GameplayStatics.SpawnSoundAtLocation` _weapondata_soundbase _returnvalue_2 (struct) 1.0 1.0 0.0 null null)
    ;[1 1 1] 현재 캐릭터일 때만
    (if (== (`self.OwnChar`) (`GameplayStatics.GetPlayerCharacter` 0))
      ;[1 1 1 1 16] 서버로(Req Shoot커스텀이벤트) 카메라 위치, Forward 길이 전달
      (`self.ReqShoot` (`PlayerCameraManager.GetCameraLocation` _returnvalue) (`self.GetActorForwardVector` _returnvalue))
      (return true))))

(fn `EventTrigger`
  (params (IsPress :type Boolean))
  (returns (bResult :type Boolean))
  (bind (_weapondata_staticmesh _weapondata_shootmontage) (break `/Game/ShootingGame/ST_Weapon` (`self.WeaponData`)))
  (`Character.PlayAnimMontage` (`self.OwnChar`) _weapondata_shootmontage 1.0 "None")
  (return true))

(fn `GetFireStartLength`
  (returns (Length :type "Float (double-precision)"))
  (bind _returnvalue (`self.GetComponentByClass` (`self.OwnChar`) "/Script/Engine.SpringArmComponent"))
  ;[1 1 1] 캐릭터의 스프링 암 컴포넌트 가져오기
  (`/Engine/EditorBlueprintResources/StandardMacros.IsValid` _returnvalue
    (:`Is Valid`
      (return (+ (`SpringArmComponent.TargetArmLength` _returnvalue) 100.0)))))

(fn `IsCanPickUp`
  (returns (IsCanPickUp :type Boolean))
  ;[1 1 1] 총을 캐릭터가 가지고 있는지 확인 후 잡을 수 있는지?
  (`/Engine/EditorBlueprintResources/StandardMacros.IsValid` (`self.OwnChar`)
    (:`Is Valid`
      (return false))
    (:`Is Not Valid`
      (return true))))

(fn `IsCanShoot`
  (returns (IsCanShoot :type Boolean))
  ;[1 1 1] Ammo가 0보다 클 때만(Pure함수)
  (return (> (`self.Ammo`) 0)))

(fn `OnRep_Ammo`
  ;[1 1 1] Ammo 확인
  (`KismetSystemLibrary.PrintString` (`KismetStringLibrary.Concat_StrStr` "Ammo : " (`KismetStringLibrary.Conv_ByteToString` (`self.Ammo`))))
  (`self.UpdateMyAmmo` (`self.Ammo`)))

(fn `SetAmmo`
  (params (Ammo :type Byte))
  (set `self.Ammo` Ammo))

(fn `UpdateMyAmmo`
  (params (Ammo :type Byte))
  (bind _returnvalue (`GameplayStatics.GetPlayerController` 0))
  (bind _ownchar (`self.OwnChar`))
  ;[1 1 1] 무기를 들고 있는 컨트롤러인지 확인
  (`/Engine/EditorBlueprintResources/StandardMacros.IsValid` _ownchar
    (:`Is Valid`
      (if (== (`Pawn.GetController` _ownchar) _returnvalue)
        ;[1 1 1] HUD에 HUDAmmo함수 전달
        (bind _asbp_shooting_hud (cast `/Game/ShootingGame/GameMode/BP_ShootingHUD` (`PlayerController.GetHUD` _returnvalue)))
        (`/Game/ShootingGame/GameMode/BP_ShootingHUD.SetHUDAmmo` _asbp_shooting_hud Ammo)))))

(fn `UseAmmo`
  (returns (IsUsed :type Boolean))
  (if (`self.IsCanShoot`)
    (set `self.Ammo` (- (`self.Ammo`) 1))
    (return true)
    (else
      (return false))))

(fn `UserConstructionScript`)