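; HUD class for the shooting game that creates the main HUD widget and sets game-only input with the cursor hidden.
; It binds to the local player state's HP, magazine and grenade dispatchers, retrying by timer until that state is available, and exposes setters that forward values to the widget.
; BindPlayerState hooks a given player's name and kill/death dispatchers to refresh the player list, retrying while the widget is invalid.
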(event `self.ReceiveBeginPlay`
  (bind _returnvalue (`GameplayStatics.GetPlayerController` 0))
  (bind _returnvalue_2 (`|CreateWidget` "/Game/ShootingGame/Widget/ShootingHudWidget.ShootingHudWidget_C"))
  (bind _output_get (set `self.HudWidget` _returnvalue_2))
  (`UserWidget.AddToViewport` _output_get 0)
  (`self.BindMyPlayerState`)
  (`WidgetBlueprintLibrary.SetInputMode_GameOnly` _returnvalue true)
  (set `PlayerController.bShowMouseCursor` false _returnvalue))

(fn `BindMyPlayerState`
  (bind _asbp_shooting_player_state (cast `/Game/ShootingGame/GameMode/BP_ShootingPlayerState` (`Controller.PlayerState` (`GameplayStatics.GetPlayerController` 0)))
    (:`then`
      (add `/Game/ShootingGame/GameMode/BP_ShootingPlayerState.EventDispatcher_UpdateMyHp` _asbp_shooting_player_state (`|CreateDelegate` :!event `SetHudHp`))
      (add `/Game/ShootingGame/GameMode/BP_ShootingPlayerState.EventDispatcher_UpdateMag` _asbp_shooting_player_state (`|CreateDelegate` :!event `SetHudMag`))
      (add `/Game/ShootingGame/GameMode/BP_ShootingPlayerState.EventDispatcher_Grenade` _asbp_shooting_player_state (`|CreateDelegate` :!event `SetHudGrenade`))
      (`self.SetHudHp` (`/Game/ShootingGame/GameMode/BP_ShootingPlayerState.CurHp` _asbp_shooting_player_state) (`/Game/ShootingGame/GameMode/BP_ShootingPlayerState.MaxHp` _asbp_shooting_player_state)))
    (:`CastFailed`
      (`KismetSystemLibrary.K2_SetTimer` null "BindMyPlayerState" 0.01))))

(fn `BindPlayerState`
  (params (PlayerState :type "/Game/ShootingGame/GameMode/BP_ShootingPlayerState Object Reference"))
  (add `/Game/ShootingGame/GameMode/BP_ShootingPlayerState.EventDispatcher_PlayerName` PlayerState (`|CreateDelegate` :!event `Update Player Name`))
  (add `/Game/ShootingGame/GameMode/BP_ShootingPlayerState.EventDispatcher_KillDeath` PlayerState (`|CreateDelegate` :!event `UpdateKillDeath`))
  (`KismetSystemLibrary.PrintString` "BindPlayerState" false false (struct :`G` 0.66 :`B` 1.0 :`A` 1.0) 60.0)
  (`self.Update Player Name` (`/Game/ShootingGame/GameMode/BP_ShootingPlayerState.UserName` PlayerState)))

(fn `SetHudAmmo`
  (params (Ammo :type Byte))
  (`/Game/ShootingGame/Widget/ShootingHudWidget.SetAmmo` (`self.HudWidget`) Ammo))

(fn `SetHudGrenade`
  (params (Grenade :type Integer))
  (`/Game/ShootingGame/Widget/ShootingHudWidget.SetGrenade` (`self.HudWidget`) Grenade))

(fn `SetHudHp`
  (params (CurHp :type "Float (double-precision)") (MaxHp :type "Float (double-precision)"))
  (`/Game/ShootingGame/Widget/ShootingHudWidget.SetHp` (`self.HudWidget`) CurHp MaxHp))

(fn `SetHudMag`
  (params (Mag :type Integer))
  (`/Game/ShootingGame/Widget/ShootingHudWidget.SetMag` (`self.HudWidget`) Mag))

(fn `Update Player Name`
  (params (UserName :type String))
  (bind _hudwidget (`self.HudWidget`))
  (`/Engine/EditorBlueprintResources/StandardMacros.IsValid` _hudwidget
    (:`Is Valid`
      (`/Game/ShootingGame/Widget/ShootingHudWidget.UpdatePlayerList` _hudwidget))
    (:`Is Not Valid`
      (`self.UpdateHud`))))

(fn `UpdateHud`
  (bind _hudwidget (`self.HudWidget`))
  (`/Engine/EditorBlueprintResources/StandardMacros.IsValid` _hudwidget
    (:`Is Valid`
      (`/Game/ShootingGame/Widget/ShootingHudWidget.UpdatePlayerList` _hudwidget))
    (:`Is Not Valid`
      (`KismetSystemLibrary.K2_SetTimer` null "UpdateHud" 0.01))))

(fn `UpdateKillDeath`
  (params (Kill :type Integer) (Death :type Integer))
  (bind _hudwidget (`self.HudWidget`))
  (`/Engine/EditorBlueprintResources/StandardMacros.IsValid` _hudwidget
    (:`Is Valid`
      (`/Game/ShootingGame/Widget/ShootingHudWidget.UpdatePlayerList` _hudwidget))
    (:`Is Not Valid`
      (`self.UpdateHud`))))

(fn `UserConstructionScript`)