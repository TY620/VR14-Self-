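; BP_LobbyPlayerState is the lobby player state that holds each player's user name for the lobby HUD.
; On BeginPlay it casts player controller 0's HUD to BP_LobbyHud and binds itself to it.
; SetUserName writes the replicated UserName, whose OnRep function fires the player name event dispatcher with the new value.
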(event `self.ReceiveBeginPlay`
  (bind _asbp_lobby_hud (cast `/Game/ShootingGame/GameMode/Lobby/BP_LobbyHud` (`PlayerController.GetHUD` (`GameplayStatics.GetPlayerController` 0))))
  (`/Game/ShootingGame/GameMode/Lobby/BP_LobbyHud.BindPlayerState` _asbp_lobby_hud self))

(fn `OnRep_UserName`
  (`KismetSystemLibrary.PrintString` "OnRepUserName" false false (struct :`G` 0.66 :`B` 1.0 :`A` 1.0) 60.0)
  (`self.EventDispatcher_PlayerName` (`self.UserName`)))

(fn `SetUserName`
  (params (UserName :type String))
  (set `self.UserName` UserName))

(fn `UserConstructionScript`)