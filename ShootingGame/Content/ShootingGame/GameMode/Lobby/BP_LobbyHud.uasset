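; Lobby HUD for the shooting game that creates the lobby widget on BeginPlay and switches to UI-only input with a visible cursor.
; BindPlayerState binds to a player state's name event dispatcher and immediately calls UpdatePlayerName with the current name.
; UpdatePlayerName refreshes the widget's player list, falling back to UpdateHud, which retries on a short timer until the widget is valid.
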(event `self.ReceiveBeginPlay`
  (bind _returnvalue (`GameplayStatics.GetPlayerController` 0))
  (bind _returnvalue_2 (`|CreateWidget` "/Game/ShootingGame/Widget/Lobby/LobbyHUDWidget.LobbyHUDWidget_C"))
  (bind _output_get (set `self.LobbyHUDWidget` _returnvalue_2))
  (`UserWidget.AddToViewport` _output_get 0)
  (`WidgetBlueprintLibrary.SetInputMode_UIOnlyEx` _returnvalue null)
  (set `PlayerController.bShowMouseCursor` true _returnvalue))

(fn `BindPlayerState`
  (params (PlayerState :type "/Game/ShootingGame/GameMode/Lobby/BP_LobbyPlayerState Object Reference"))
  (add `/Game/ShootingGame/GameMode/Lobby/BP_LobbyPlayerState.EventDispatcher_PlayerName` PlayerState (`|CreateDelegate` :!event `UpdatePlayerName`))
  (`KismetSystemLibrary.PrintString` "BindPlayerState" false false (struct :`G` 0.66 :`B` 1.0 :`A` 1.0) 60.0)
  (`self.UpdatePlayerName` (`/Game/ShootingGame/GameMode/Lobby/BP_LobbyPlayerState.UserName` PlayerState)))

(fn `UpdateHud`
  (bind _lobbyhudwidget (`self.LobbyHUDWidget`))
  (`/Engine/EditorBlueprintResources/StandardMacros.IsValid` _lobbyhudwidget
    (:`Is Valid`
      (`/Game/ShootingGame/Widget/Lobby/LobbyHUDWidget.UpdatePlayerList` _lobbyhudwidget))
    (:`Is Not Valid`
      (`KismetSystemLibrary.K2_SetTimer` null "UpdateHud" 0.01))))

(fn `UpdatePlayerName`
  (params (UserName :type String))
  (bind _lobbyhudwidget (`self.LobbyHUDWidget`))
  (`KismetSystemLibrary.PrintString` (`KismetStringLibrary.Concat_StrStr` "UpdatePlayerName - " UserName) false false (struct :`G` 0.66 :`B` 1.0 :`A` 1.0) 60.0)
  (`/Engine/EditorBlueprintResources/StandardMacros.IsValid` _lobbyhudwidget
    (:`Is Valid`
      (`/Game/ShootingGame/Widget/Lobby/LobbyHUDWidget.UpdatePlayerList` _lobbyhudwidget))
    (:`Is Not Valid`
      (`self.UpdateHud`))))

(fn `UserConstructionScript`)