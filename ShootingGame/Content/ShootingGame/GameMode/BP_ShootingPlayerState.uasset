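; Player state for the shooting game that holds a player's current and max HP, starting at full health on BeginPlay.
; AddDamage subtracts from CurHP, a RepNotify variable whose OnRep prints the new value for debugging.
; The OnRep also fires the UpdateMyHP dispatcher, but only when this state's pawn is player 0's pawn, so listeners receive just the local player's health.
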(event `self.ReceiveBeginPlay`
  (set `self.CurHP` (`self.MaxHP`)))

(fn `AddDamage`
  (params (Damage :type "Float (double-precision)"))
  ;[1 1 1] Notify로 설정하면 OnRep_CurHP 생성
  (set `self.CurHP` (- (`self.CurHP`) Damage)))

(fn `OnRep_CurHP`
  ;[1 1 1] 리플리케이트 되야되는 변수
  (`KismetSystemLibrary.PrintString` (`KismetStringLibrary.Concat_StrStr` "OnRep_CurHP : " (`KismetStringLibrary.Conv_DoubleToString` (`self.CurHP`))))
  (if (== (`GameplayStatics.GetPlayerPawn` 0) (`self.PawnPrivate`))
    (`self.EventDispatcher_UpdateMyHP` (`self.CurHP`) (`self.MaxHP`))))

(fn `UserConstructionScript`)