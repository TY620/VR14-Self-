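; Player controller for the shooting game that passes the player's name to their player state when a pawn is possessed.
; On possess, it calls ResClientPossess, which reads PlayerName from BP_ShootingGameInstance and sends it toward the server through ReqChangeUserName.
; ReqChangeUserName then applies the name to BP_ShootingPlayerState with SetUserName.
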(event `ResClientPossess`
  (`KismetSystemLibrary.PrintString` "ResClientPossess" true true (struct :`G` 0.66 :`B` 1.0 :`A` 1.0) 60.0)
  ;[1 1 1] 이름을 서버로
  (bind _asbp_shooting_game_instance (cast `/Game/ShootingGame/GameMode/BP_ShootingGameInstance` (`GameplayStatics.GetGameInstance`)))
  (`self.ReqChangeUserName` (`/Game/ShootingGame/GameMode/BP_ShootingGameInstance.PlayerName` _asbp_shooting_game_instance)))

(event `self.ReceivePossess`
  (params (PossessedPawn :type "Pawn Object Reference"))
  (`KismetSystemLibrary.PrintString` (`KismetStringLibrary.Concat_StrStr` "PlayerController OnPossess - " (`KismetSystemLibrary.GetDisplayName` PossessedPawn)) false false (struct :`G` 0.66 :`B` 1.0 :`A` 1.0) 60.0)
  (`self.ResClientPossess`))

(event `ReqChangeUserName`
  (params (UserName :type String))
  (bind _asbp_shooting_player_state (cast `/Game/ShootingGame/GameMode/BP_ShootingPlayerState` (`self.PlayerState`)))
  (`/Game/ShootingGame/GameMode/BP_ShootingPlayerState.SetUserName` _asbp_shooting_player_state UserName))

(fn `UserConstructionScript`)