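; Grenade actor for a shooting game that, on the server, explodes three seconds after spawning.
; ResExplosion spawns the particle effect and sound, then destroys the actor, without calling the damage function.
; ApplyGrenadeDamage, not called in this graph, applies radial falloff damage sized by the Sphere component's radius, then calls PushCharacter.
; PushCharacter launches overlapping Characters away from the center with impulses that weaken linearly with distance.
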(event `self.ReceiveBeginPlay`
  (`/Engine/EditorBlueprintResources/ActorMacros.Switch Has Authority`
    (:`Authority`
      (`KismetSystemLibrary.Delay` 3.0)
      (`self.ResExplosion`))))

(event `ResExplosion`
  (bind (_returnvalue_location _returnvalue_rotation) (`KismetMathLibrary.BreakTransform` (`self.GetTransform`)))
  (`GameplayStatics.SpawnEmitterAtLocation` "/Game/StarterContent/Particles/P_Explosion.P_Explosion" _returnvalue_location _returnvalue_rotation (5.0 5.0 5.0))
  (`GameplayStatics.SpawnSoundAtLocation` "/Game/StarterContent/Audio/Explosion_Cue.Explosion_Cue" _returnvalue_location (struct) 1.0 1.0 0.0 null null)
  (`self.K2_DestroyActor`))

(fn `ApplyGrenadeDamage`
  (bind _sphereradius (`SphereComponent.SphereRadius` (`self.Sphere`)))
  (`GameplayStatics.ApplyRadialDamageWithFalloff` :`BaseDamage` 100.0 :`MinimumDamage` 10.0 :`Origin` (`SceneComponent.K2_GetComponentLocation` (`self.Sphere`)) :`DamageInnerRadius` (* _sphereradius 0.2) :`DamageOuterRadius` _sphereradius :`DamageFalloff` 0.1 :`DamageCauser` self :`InstigatedByController` (`self.Controller`))
  (`self.PushCharacter`))

(fn `CalcPushImpulse`
  (params (Start :type "Vector Structure (by ref)") (Target :type "Vector Structure (by ref)"))
  (returns (ReturnValue :type "Vector Structure"))
  (return (* (`KismetMathLibrary.GetForwardVector` (`KismetMathLibrary.FindLookAtRotation` Start Target)) (* (- 1.0 (/ (`KismetMathLibrary.Vector_Distance` Start Target) (`SphereComponent.SphereRadius` (`self.Sphere`)))) 200000.0))))

(fn `PushCharacter`
  (for _array_element (`PrimitiveComponent.GetOverlappingActors` (`self.Sphere`) "/Script/Engine.Character")
    (bind `_as캐릭터` (cast `Character` _array_element))
    (`CharacterMovementComponent.AddImpulse` (`Character.CharacterMovement` `_as캐릭터`) (`self.CalcPushImpulse` (`SceneComponent.K2_GetComponentLocation` (`self.Sphere`)) (`self.K2_GetActorLocation` `_as캐릭터`)) false)))

(fn `UserConstructionScript`)