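; BP_Timer is an actor that shows a running minutes:seconds timer on a TextRender component.
; While IsPlay is set, Tick accumulates delta time at ten times real speed and displays it, using FloatToStr00 to floor and zero-pad each field.
; EventComponent's play and stop dispatchers toggle IsPlay, as do DoPlay and DoStop overrides that also call their parent versions.
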(event `self.ReceiveTick`
  (params (DeltaSeconds :type "Float (single-precision)"))
  (if (`self.IsPlay`)
    (bind _output_get (set `self.TotalDelta` (+ (* DeltaSeconds 10.0) (`self.TotalDelta`))))
    (bind _str00 (`self.FloatToStr00` (/ _output_get 60.0)))
    (bind _str00_2 (`self.FloatToStr00` (mod _output_get 60.0)))
    (`TextRenderComponent.K2_SetText` (`self.TextRender`) (`KismetTextLibrary.Conv_StringToText` (`KismetStringLibrary.Concat_StrStr` _str00 ":" _str00_2)))))

(event `self.EventComponent.NewEventDispatcher_DoPlay`
  (set `self.IsPlay` true))

(event `self.EventComponent.NewEventDispatcher_DoStop`
  (set `self.IsPlay` false))

(fn `DoPlay`
  (`parent.DoPlay`)
  (set `self.IsPlay` true))

(fn `DoStop`
  (`parent.DoStop`)
  (set `self.IsPlay` false))

(fn `FloatToStr00`
  (params (Number :type "Float (double-precision)"))
  (returns (Str00 :type String))
  (bind _returnvalue (`KismetMathLibrary.FFloor` Number))
  (if (< _returnvalue 10.0)
    (return (`KismetStringLibrary.Concat_StrStr` "0" (`KismetStringLibrary.Conv_IntToString` _returnvalue)))
    (else
      (return (`KismetStringLibrary.Conv_IntToString` _returnvalue)))))

(fn `UserConstructionScript`)