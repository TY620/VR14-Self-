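; Actor Blueprint that slides its Sphere back and forth along the relative X axis with a timeline.
; EventComponent's play dispatcher plays or reverses the timeline based on IsMoveRight, and its stop dispatcher halts it.
; Each finish flips IsMoveRight and re-enters that branch, so the motion loops until stopped.
; DoPlay and DoStop call their parent versions, then the empty EventStart and EventEnd hooks.
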(event `EventStart`)

(event `EventEnd`)

(event `self.ReceiveBeginPlay`)

(event `self.EventComponent.NewEventDispatcher_DoPlay`
  (if (`self.IsMoveRight`) :!label _label
    (bind (_direction _value) (`Timeline|타임라인` :!label _label_2)
      (:`Update`
        (`SceneComponent.K2_SetRelativeLocation` (`self.Sphere`) (`KismetMathLibrary.MakeVector` (* _value 100.0)) false false))
      (:`Finished`
        (set `self.IsMoveRight` (not (`self.IsMoveRight`)))
        (goto _label)))
    (else
      (goto _label_2 :!via `Reverse`))))

(event `self.EventComponent.NewEventDispatcher_DoStop`
  (goto _label_2 :!via `Stop`))

(fn `DoPlay`
  (`parent.DoPlay`)
  (`self.EventStart`))

(fn `DoStop`
  (`parent.DoStop`)
  (`self.EventEnd`))

(fn `UserConstructionScript`)